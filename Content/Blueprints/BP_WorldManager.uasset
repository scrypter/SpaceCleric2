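; BP_WorldManager drives the time of day and the lighting that follows it.
; On BeginPlay it runs Init and hands the directional sun light to LightManager.
; Each tick it advances TimeManager, feeds the current hour to LightManager, then refreshes the SkySphere sun direction.
; It also prints the hour on screen every frame as debug output.
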(event `self.ReceiveBeginPlay`
  (`self.Init`)
  (`LightManager.SetSun` (`self.LightManager`) (`self.SunDirectionalLight`)))

(event `self.ReceiveTick`
  (params (DeltaSeconds :type "Float (single-precision)"))
  (set `self.DeltaTime` DeltaSeconds)
  (`|ExecutionSequence`
    (:`then_0`
      (`TimeManager.Update` (`self.TimeManager`) (`self.DeltaTime`)))
    (:`then_1`
      (bind _returnvalue (`TimeManager.GetHour` (`self.TimeManager`)))
      (`LightManager.Update` (`self.LightManager`) _returnvalue)
      (`KismetSystemLibrary.PrintString` (`KismetStringLibrary.Conv_DoubleToString` _returnvalue) true true (struct :`G` 0.66 :`B` 1.0 :`A` 1.0) 0.0001))
    (:`then_2`
      (`/Engine/EngineSky/BP_Sky_Sphere.UpdateSunDirection` (`self.SkySphere`)))))

(fn `UserConstructionScript`)